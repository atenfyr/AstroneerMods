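; QTPrinter_BP is a printer item in the BackpackPrinterMod that takes its blueprint list from the mod's actor.
; On BeginPlay it finds the AtenBPMActor in the level and passes that actor's AllBlueprints to its Printer through SetBlueprints.
; The pickup, drop, hit and slot-placement events, along with the construction script, only call their parent implementations.
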(event EventBeginPlay
  (|CallParentFunction)
  (bind _returnvalue (Actor|GetActorOfClass "/Game/Atenfyr/BackpackPrinterMod/AtenBPMActor.AtenBPMActor_C"))
  (Class|PrinterComponent|SetBlueprints (Variables|Default|GetPrinter) (Variables|/Game/Atenfyr/BackpackPrinterMod/AtenBPMActor.AtenBPMActor_C|GetAllBlueprints _returnvalue)))

(event EventPlacedinSlot
  (params (Slot :type Slot%20Reference%20Structure) (FromTool :type Boolean) (SlottedDuringInitialization :type Boolean))
  (|CallParentFunction Slot FromTool SlottedDuringInitialization))

(event EventPickedUpfromWorld
  (|CallParentFunction))

(event EventDroppedinWorld
  (params (Component :type Primitive%20Component%20Object%20Reference) (terrainComponent :type Boolean) (Point :type Vector :default "0, 0, 0") (Normal :type Vector :default "0, 0, 0"))
  (|CallParentFunction Component terrainComponent Point Normal))

(event Collision|EventHit
  (params (MyComp :type Primitive%20Component%20Object%20Reference) (Other :type Actor%20Object%20Reference) (OtherComp :type Primitive%20Component%20Object%20Reference) (bSelfMoved :type Boolean) (HitLocation :type Vector :default "0, 0, 0") (HitNormal :type Vector :default "0, 0, 0") (NormalImpulse :type Vector :default "0, 0, 0") (Hit :type Hit%20Result%20Structure%20%28by%20ref%29))
  (|CallParentFunction MyComp Other OtherComp bSelfMoved HitLocation HitNormal NormalImpulse Hit))

(fn ConstructionScript
  (|CallParentFunction))